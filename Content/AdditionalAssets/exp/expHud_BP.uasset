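; HUD Blueprint that manages opening and closing the stat choice screen.
; BeginPlay creates one StatChoice_wbp widget for the owning player and keeps it for reuse.
; OpenStats adds it to the viewport, enables cursor and click events, and disables input on the controlled pawn.
; Closestats removes the widget and restores pawn input, but leaves the cursor and click events enabled.
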(event EventBeginPlay
  (bind _returnvalue (UserInterface|CreateWidget "/Game/AdditionalAssets/exp/StatChoice_wbp.StatChoice_wbp_C" (Game|Player|GetOwningPlayerController)))
  (Variables|Default|SetStatwidgetRef _returnvalue))

(event EventOpenStats
  (bind _returnvalue (Game|Player|GetOwningPlayerController))
  (UserInterface|Viewport|AddtoViewport (Variables|Default|GetStatwidgetRef) 0)
  (Variables|/Script/Engine.PlayerController|SetbShowMouseCursor _returnvalue true)
  (Variables|/Script/Engine.PlayerController|SetbEnableClickEvents _returnvalue true)
  (Input|DisableInput (Pawn|GetControlledPawn _returnvalue) _returnvalue))

(event EventClosestats
  (bind _returnvalue (Game|Player|GetOwningPlayerController))
  (Widget|RemovefromParent (Variables|Default|GetStatwidgetRef))
  (Variables|/Script/Engine.PlayerController|SetbShowMouseCursor _returnvalue true)
  (Variables|/Script/Engine.PlayerController|SetbEnableClickEvents _returnvalue true)
  (Input|EnableInput (Pawn|GetControlledPawn _returnvalue) _returnvalue))

(fn ConstructionScript)