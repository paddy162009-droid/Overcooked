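; BP_CheckpointVolume is a checkpoint trigger that updates the respawn point when player 0's pawn enters its Box.
; BeginPlay caches the RespawnManager_BPC component from the game mode, and the overlap event passes it the pawn's current transform, not the volume's.
; If IsSingleUse is set, the volume destroys itself after updating.
; An older route through BP_CombatPlayerController's SetRespawnTransform remains in the graph but never runs.
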(event OnComponentBeginOverlap(Box)
  (params (OverlappedComponent :type Primitive%20Component%20Object%20Reference) (OtherActor :type Actor%20Object%20Reference) (OtherComp :type Primitive%20Component%20Object%20Reference) (OtherBodyIndex :type Integer) (bFromSweep :type Boolean) (SweepResult :type Hit%20Result%20Structure%20%28by%20ref%29))
  (if (== OtherActor (Game|Player|GetPlayerPawn 0))
    (bind _respawnmanagerref (Variables|Default|GetRespawnManagerRef)
      (:then
        (Default|UpdateRespawnPoint _respawnmanagerref (Transformation|GetActorTransform OtherActor))
        (if (Variables|Default|GetIsSingleUse?)
          (Actor|DestroyActor)))
      (:else))))

(event EventBeginPlay
  (Variables|Default|SetRespawnManagerRef (Actor|GetComponentbyClass (Game|GetGameMode) "/Game/AdditionalAssets/RespawnManager_BPC.RespawnManager_BPC_C")))

(fn ConstructionScript)